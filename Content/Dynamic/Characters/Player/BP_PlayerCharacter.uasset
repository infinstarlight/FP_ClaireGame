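; Player character with a grappling-rope swing, reading hook state from BP_PlayerController.
; Tick stretches the Hook cable between hook point and hand socket, applying a velocity-dot-product force along the rope and full air control while CanHook is false.
; A looping timer sphere-traces below the character to set the controller's IsInAir flag; landing breaks the rope link.
; SwingInRotation, not called here, orients NewCapsule, the mesh's runtime parent, along the rope during airborne swings.
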(event `self.ReceiveBeginPlay`
  (bind _hook (`self.Hook`))
  (`SceneComponent.SetVisibility` _hook false false)
  (set `CableComponent.EndLocation` (0.0 0.0 0.0) _hook)
  (`SceneComponent.K2_AttachToComponent` (`self.Mesh`) (`self.NewCapsule`) "None" "KeepWorld" "KeepWorld" "KeepWorld" true)
  (`KismetSystemLibrary.K2_SetTimer` null "PlayerIsFalling" 0.3 true))

(event `self.ReceiveTick`
  (params (DeltaSeconds :type "Float (single-precision)"))
  (`self.ThrowRope`))

(event `self.OnLanded`
  (params (Hit :type "HitResult Structure (by ref)"))
  (`/Game/Dynamic/Characters/Player/BP_PlayerController.BreakRopeLink` (cast `/Game/Dynamic/Characters/Player/BP_PlayerController` (`GameplayStatics.GetPlayerController` 0) :!pure true)))

(fn `PlayerIsFalling`
  (bind (_returnvalue_x _returnvalue_y _returnvalue_z) (`KismetMathLibrary.BreakVector` (`self.K2_GetActorLocation`)))
  (bind _asbp_player_controller (cast `/Game/Dynamic/Characters/Player/BP_PlayerController` (`GameplayStatics.GetPlayerController` 0) :!pure true))
  (bind _returnvalue (`KismetMathLibrary.MakeVector` _returnvalue_x _returnvalue_y (- _returnvalue_z 90.0)))
  (bind (_outhit _returnvalue_2) (`KismetSystemLibrary.SphereTraceSingle` _returnvalue _returnvalue 50.0 "TraceTypeQuery1"))
  (if _returnvalue_2
    (set `/Game/Dynamic/Characters/Player/BP_PlayerController.IsInAir?` false _asbp_player_controller)
    (else
      (set `/Game/Dynamic/Characters/Player/BP_PlayerController.IsInAir?` true _asbp_player_controller))))

(fn `SwingInRotation`
  (bind _asbp_player_controller (cast `/Game/Dynamic/Characters/Player/BP_PlayerController` (`GameplayStatics.GetPlayerController` 0) :!pure true))
  (bind _returnvalue (`KismetMathLibrary.Normal` (- (`/Game/Dynamic/Characters/Player/BP_PlayerController.HookPoint` _asbp_player_controller) (`self.K2_GetActorLocation`))))
  (if (and (`/Game/Dynamic/Characters/Player/BP_PlayerController.IsPlayerHooked?` _asbp_player_controller) (`/Game/Dynamic/Characters/Player/BP_PlayerController.IsInAir?` _asbp_player_controller))
    (`SceneComponent.K2_SetWorldRotation` (`self.NewCapsule`) (`KismetMathLibrary.MakeRotFromZY` _returnvalue (* (`KismetMathLibrary.Cross_VectorVector` (`KismetMathLibrary.Normal` (`self.GetVelocity`)) _returnvalue) -1.0)) false false)
    (else
      (`SceneComponent.K2_SetWorldRotation` (`self.Hook`) (`KismetMathLibrary.MakeRotator` 0.0 0.0 (.yaw (`SceneComponent.K2_GetComponentRotation` (`self.NewCapsule`)))) false false))))

(fn `ThrowRope`
  (bind _returnvalue_location (`KismetMathLibrary.BreakTransform` (`SceneComponent.GetSocketTransform` (`self.Mesh`) (`self.HandSocket`) "RTS_Actor")))
  (bind _asbp_player_controller (cast `/Game/Dynamic/Characters/Player/BP_PlayerController` (`GameplayStatics.GetPlayerController` 0) :!pure true))
  (bind _returnvalue (- (`self.K2_GetActorLocation`) (`/Game/Dynamic/Characters/Player/BP_PlayerController.HookPoint` (cast `/Game/Dynamic/Characters/Player/BP_PlayerController` (`GameplayStatics.GetPlayerController` 0) :!pure true))))
  (if (`/Game/Dynamic/Characters/Player/BP_PlayerController.IsPlayerHooked?` _asbp_player_controller)
    (`SceneComponent.K2_SetWorldLocation` (`self.Hook`) (`/Game/Dynamic/Characters/Player/BP_PlayerController.HookPoint` _asbp_player_controller) false false)
    (set `CableComponent.EndLocation` _returnvalue_location (`self.Hook`))
    (if (not (`/Game/Dynamic/Characters/Player/BP_PlayerController.CanHook?` (cast `/Game/Dynamic/Characters/Player/BP_PlayerController` (`GameplayStatics.GetPlayerController` 0) :!pure true)))
      (`CharacterMovementComponent.AddForce` (`self.CharacterMovement`) (* (* (`KismetMathLibrary.Normal` _returnvalue) (`KismetMathLibrary.Dot_VectorVector` (`self.GetVelocity`) _returnvalue)) (`self.RopeForce`)))
      (set `CableComponent.CableLength` (- (`/Game/Dynamic/Characters/Player/BP_PlayerController.RopeDistanceFromActor` (cast `/Game/Dynamic/Characters/Player/BP_PlayerController` (`GameplayStatics.GetPlayerController` 0) :!pure true)) 300.0) (`self.Hook`))
      (set `CharacterMovementComponent.AirControl` 1.0 (`self.CharacterMovement`)))))

(fn `UserConstructionScript`)